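; BP_Object is an interactable actor that tracks when it can be interacted with and can be reset to its starting placement.
; Begin and end overlap toggle its MCanInteract flag for any actor, and for PC_Main also mirror the flag and call CanInteractWidgetCall.
; The construction script clears the flag and caches the starting transform, which ResetObject restores while clearing the flag again.
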(event Collision|EventActorBeginOverlap
  (params (OtherActor :type Actor%20Object%20Reference))
  (Variables|State|SetM%20CanInteract true)
  (bind _aspc_main (Utilities|Casting|CastToPC_Main OtherActor))
  (Variables|/Game/Blueprints/Players/PC_Main.PC_Main_C|SetM%20CanInteract _aspc_main true)
  (Default|CanInteractWidgetCall _aspc_main))

(event Collision|EventActorEndOverlap
  (params (OtherActor :type Actor%20Object%20Reference))
  (Variables|State|SetM%20CanInteract false)
  (bind _aspc_main (Utilities|Casting|CastToPC_Main OtherActor))
  (Variables|/Game/Blueprints/Players/PC_Main.PC_Main_C|SetM%20CanInteract _aspc_main false)
  (Default|CanInteractWidgetCall _aspc_main))

(fn ConstructionScript
  (Variables|State|SetM%20CanInteract false)
  (Variables|Components|SetM%20StartTransform (Transformation|GetActorTransform self)))

(fn ResetObject
  (Variables|State|SetM%20CanInteract false)
  (Transformation|SetActorTransform (Variables|Components|GetM%20StartTransform)))