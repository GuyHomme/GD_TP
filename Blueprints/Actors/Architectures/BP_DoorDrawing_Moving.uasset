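; BP_DoorDrawing_Moving is a door drawing actor that rides on the wall it follows, presumably a moving one.
; On BeginPlay it runs the parent logic, attaches to MWallFollowed and takes its relative location from that wall's MDoorLocations array at MIndex.
; It then makes a component attachment to the wall's PlatformMesh, keeping relative transforms.
; The construction script only calls the parent.
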(event EventBeginPlay
  (|CallParentFunction)
  (Transformation|AttachActorToActor (Variables|Default|GetM%20WallFollowed) "None" "KeepRelative" "KeepRelative" "KeepRelative" true)
  (Transformation|SetActorRelativeLocation (Utilities|Array|Get(acopy) (Variables|/Game/Blueprints/Actors/Architectures/BP_PlatMovingWall_OffensiveDoorDrawing.BP_PlatMovingWall_OffensiveDoorDrawing_C|GetM%20DoorLocations (Variables|Default|GetM%20WallFollowed)) (Variables|Default|GetM%20Index)))
  (Transformation|AttachComponentToComponent (Variables|/Game/Blueprints/Actors/Architectures/BP_TypePlatform.BP_TypePlatform_C|GetPlatformMesh (Variables|Default|GetM%20WallFollowed)) "None" "KeepRelative" "KeepRelative" "KeepRelative" true))

(fn ConstructionScript
  (|CallParentFunction))