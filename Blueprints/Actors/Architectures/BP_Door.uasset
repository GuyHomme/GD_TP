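; Door actor that lifts open once a required number of conditions is met, optionally in a set caller order.
; Callers increment or decrement the verified count, with opening also gated by a CanOpen flag and any decrement closing an open door.
; A timeline lerps the mesh's relative Z, reversing to close, while audio plays and follower objects are told to mirror each change.
; ResetDoor closes it and clears the count.
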(event Custom|OpenDoor
  (bind _audio (Variables|Default|GetAudio))
  ;[1 1 1] Animations
  (Variables|Components|SetM%20Closed false)
  (if (Audio|Components|Audio|IsPlaying _audio)
    (Audio|Components|Audio|Stop _audio))
  (Audio|Components|Audio|Play _audio 0.0)
  (for _array_element (Variables|Components|GetM%20Followers)
    (Default|FollowMyOpening _array_element))
  (bind _lift (Timeline|Opening Play)
    (:Update
      (Transformation|SetRelativeLocation (Variables|Default|GetDoor) (Math|Vector|Lerp(Vector) "0, 0, 0" (Math|Vector|MakeVector 0.0 0.0 (Utilities|GETDOORZLIFT)) _lift) false false)
      (Audio|Components|Audio|FadeOut (Variables|Default|GetAudio) (/ (Components|Timeline|GetTimelineLength (Variables|Default|GetOpening)) 2.0) 0.0 :!class /Script/Engine.AudioComponent))))

(event Custom|OneLessCondition
  (params (Caller :type BP%20Object%20Object%20Reference))
  (bind _m_verifiedcondition (Variables|Components|GetM%20VerifiedCondition))
  ;[1 1 1] Conditions and INC/DECrementation
  (if (> _m_verifiedcondition 0)
    (Math|Integer|DecrementInt _m_verifiedcondition
      (:%20%20
        (if (not (Variables|Components|GetM%20Closed))
          (CallFunction|CloseDoor))))))

(event Custom|CloseDoor
  (bind _audio (Variables|Default|GetAudio))
  ;[1 1 1] Animations
  (Variables|Components|SetM%20Closed true)
  (if (Audio|Components|Audio|IsPlaying _audio)
    (Audio|Components|Audio|Stop _audio))
  (Audio|Components|Audio|Play _audio 0.0)
  (for _array_element (Variables|Components|GetM%20Followers)
    (Default|FollowMyClosing _array_element))
  (bind _lift (Timeline|Opening Reverse)
    (:Update
      (Transformation|SetRelativeLocation (Variables|Default|GetDoor) (Math|Vector|Lerp(Vector) "0, 0, 0" (Math|Vector|MakeVector 0.0 0.0 (Utilities|GETDOORZLIFT)) _lift) false false)
      (Audio|Components|Audio|FadeOut (Variables|Default|GetAudio) (/ (Components|Timeline|GetTimelineLength (Variables|Default|GetOpening)) 2.0) 0.0 :!class /Script/Engine.AudioComponent))))

(event Custom|TryOpening
  (params (Can%20Open :type Boolean))
  ;[1 1 1] Tries
  (if Can%20Open
    (CallFunction|OpenDoor)))

(event Custom|OneMoreCondition
  (params (Caller :type BP%20Object%20Object%20Reference) (CanOpen :type Boolean))
  ;[1 1 1] Conditions and INC/DECrementation
  (if (Variables|Components|GetM%20Order)
    (if (== (Utilities|Array|Get(acopy) (Variables|Components|GetM%20OrderArray) (Variables|Components|GetM%20VerifiedCondition)) (Variables|/Game/Blueprints/Actors/Interactables/BP_Object.BP_Object_C|GetM%20Index Caller))
      (bind _result (Math|Integer|IncrementInt (Variables|Components|GetM%20VerifiedCondition) :!label _label)
        (:%20%20
          (CallFunction|TryOpening (and (== (Variables|Components|GetM%20NbConditions) _result) CanOpen)))))
    (else
      (goto _label))))

(fn ConstructionScript
  (Variables|Components|SetM%20VerifiedCondition 0)
  (Variables|Components|SetM%20Closed true))

(fn ResetDoor
  (CallFunction|CloseDoor)
  (Variables|Components|SetM%20VerifiedCondition 0)
  (Variables|Components|SetM%20Closed true))